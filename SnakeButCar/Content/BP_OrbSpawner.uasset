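; Orb spawner actor that places a BP_Orbs pickup at a random spot when play begins.
; SpawnPickUp derives random X and Y from the SpawnArea box's scaled extent, without adding its X/Y location, and takes Z from its world height.
; Each new orb receives a reference back to the spawner.
; BeginPlay then broadcasts OnOrbSpawned with the BPOrb variable, which this graph never assigns.
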(event EventBeginPlay
  (CallFunction|SpawnPickUp)
  (Default|CallOnOrbSpawned (Variables|Default|GetBP_Orb)))

(fn ConstructionScript)

(fn SpawnPickUp
  (bind _spawnarea (Variables|Default|GetSpawnArea))
  (bind _returnvalue (Components|Box|GetScaledBoxExtent _spawnarea))
  (bind _returnvalue_2 (Game|SpawnActorfromClass "/Game/BP_Orbs.BP_Orbs_C" (Math|Transform|MakeTransform (Math|Vector|MakeVector (Math|Random|RandomFloatinRange (stale _result) (.x _returnvalue)) (Math|Random|RandomFloatinRange (stale _result) (.y _returnvalue)) (.z (Transformation|GetWorldLocation _spawnarea))) "0, 0, 0" "1.000000,1.000000,1.000000") "Undefined" "MultiplyWithRoot" 0 0 0))
  (Variables|/Game/BP_Orbs.BP_Orbs_C|SetBP_OrbSpawner _returnvalue_2 self))